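; BP_P38 is a player-flyable P-38 aircraft pawn with simple arcade controls that can fire rockets.
; Thrust input accumulates a clamped Speed, which scales forward movement input each tick and is passed to a SceneRotatorComponent that has both propellers registered at BeginPlay.
; Pitch and roll axes rotate the actor locally, scaled by delta time.
; Fire spawns a BP_Rocket at the plane's own transform.
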(event EventTick
  (params (DeltaSeconds :type Float%20%28single-precision%29))
  (Pawn|Input|AddMovementInput (* (Transformation|GetActorForwardVector) (* (Utilities|Time|GetWorldDeltaSeconds) (Variables|Default|GetSpeed))) 1.0 false)
  (Variables|/Game/Blueprints/SceneRotatorComponent.SceneRotatorComponent_C|SetSpeed (Variables|Default|GetSceneRotatorComponent) (Variables|Default|GetSpeed)))

(event EventBeginPlay
  (bind _scenerotatorcomponent (Variables|Default|GetSceneRotatorComponent))
  (bind _scenecomponents (Variables|/Game/Blueprints/SceneRotatorComponent.SceneRotatorComponent_C|GetSceneComponents _scenerotatorcomponent))
  (Utilities|Array|Add _scenecomponents (Variables|Default|GetPropeller_Left))
  (Utilities|Array|Add _scenecomponents (Variables|Default|GetPropeller_Right)))

(event Input|ActionEvents|InputActionFire
  (params (Key :type Key%20Structure :default "None"))
  (:Pressed
    (CallFunction|Fire)))

(event Input|AxisEvents|InputAxisPitch
  (params (AxisValue :type Float%20%28single-precision%29))
  (Transformation|AddActorLocalRotation (Math|Rotator|MakeRotator 0.0 (* (Math|Float|Clamp(Float) AxisValue -1.0) (Utilities|Time|GetWorldDeltaSeconds) 4e+01) 0.0) false false))

(event Input|AxisEvents|InputAxisRoll
  (params (AxisValue :type Float%20%28single-precision%29))
  (Transformation|AddActorLocalRotation (Math|Rotator|MakeRotator (* (Math|Float|Clamp(Float) AxisValue -1.0) (Utilities|Time|GetWorldDeltaSeconds) 4e+01) 0.0 0.0) false false))

(event Input|AxisEvents|InputAxisEngineThrust
  (params (AxisValue :type Float%20%28single-precision%29))
  (Variables|Default|SetSpeed (Math|Float|Clamp(Float) (+ (Variables|Default|GetSpeed) (* (Math|Float|Clamp(Float) AxisValue -1.0) 2.0)) 0.0 5e+02)))

(fn ConstructionScript)

(fn Fire
  (Game|SpawnActorfromClass "/Game/Blueprints/BP_Rocket.BP_Rocket_C" (Transformation|GetActorTransform) "Undefined" "MultiplyWithRoot" 0 0))